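; Player-controlled character for Task 05 that loops along a Trajectory spline and launches physics balls with an aimed landing preview.
; Tick advances a wrapped spline time, scaled by a keyboard-adjustable speed multiplier.
; Holding left mouse spawns a hit marker that follows a debug-drawn projectile path prediction.
; Releasing launches a ball using the same velocity, with ball and marker lifespans derived from the predicted flight time.
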(event EventBeginPlay)

(event EventTick
  (params (DeltaSeconds :type Float%20%28single-precision%29))
  (CallFunction|HandleMovement DeltaSeconds)
  (CallFunction|UpdatePredictionPath))

(event Input|KeyboardEvents|Equals
  (params (Key :type Key%20Structure :default "None"))
  (:Pressed
    (Variables|Default|SetSpeedMultiplier (Math|Float|Clamp(Float) (+ (Variables|Default|GetSpeedMultiplier) 0.1) 0.0 2.0))))

(event Input|KeyboardEvents|Hyphen
  (params (Key :type Key%20Structure :default "None"))
  (:Pressed
    (Variables|Default|SetSpeedMultiplier (Math|Float|Clamp(Float) (- (Variables|Default|GetSpeedMultiplier) 0.1) 0.0 2.0))))

(event Input|KeyboardEvents|Add
  (params (Key :type Key%20Structure :default "None"))
  (:Pressed
    (Variables|Default|SetSpeedMultiplier (Math|Float|Clamp(Float) (+ (Variables|Default|GetSpeedMultiplier) 0.1) 0.0 2.0))))

(event Input|KeyboardEvents|Subtract
  (params (Key :type Key%20Structure :default "None"))
  (:Pressed
    (Variables|Default|SetSpeedMultiplier (Math|Float|Clamp(Float) (- (Variables|Default|GetSpeedMultiplier) 0.1) 0.0 2.0))))

(event Input|MouseEvents|LeftMouseButton
  (params (Key :type Key%20Structure :default "None"))
  (:Pressed
    (Variables|Default|SetbShouldUpdatePrediction true)
    (bind _returnvalue (Game|SpawnActorfromClass "/Game/Task_05/BP_HitPlace.BP_HitPlace_C" (Math|Transform|MakeTransform "0, 0, 0" "0, 0, 0" "1.000000,1.000000,1.000000") "AlwaysSpawn" "MultiplyWithRoot" 0 0))
    (Variables|Default|SetHitPlace _returnvalue))
  (:Released
    (Variables|Default|SetbShouldUpdatePrediction false)
    (bind _returnvalue_2 (Game|SpawnActorfromClass "/Game/Task_05/BP_PhysicBall.BP_PhysicBall_C" (Math|Transform|MakeTransform (Transformation|GetWorldLocation (Variables|Default|GetProjectileSpawnPoint)) (Transformation|GetWorldRotation (Variables|Default|GetProjectileSpawnPoint)) "1.000000,1.000000,1.000000") "Undefined" "MultiplyWithRoot" 0 0))
    (Actor|SetLifeSpan _returnvalue_2 (+ (Variables|Default|GetLastPredictionPathDuration) 0.5))
    (Physics|AddImpulse (Variables|/Game/Task_05/BP_PhysicBall.BP_PhysicBall_C|GetSphere _returnvalue_2) (* (Math|Vector|GetForwardVector (Variables|Default|GetProjectileSpawnPoint)) (Variables|Default|GetLaunchVelocity)) "None" true)
    (Actor|SetLifeSpan (Variables|Default|GetHitPlace) (Variables|Default|GetLastPredictionPathDuration))))

(fn ConstructionScript)

(fn HandleMovement
  (params (DeltaSeconds :type Float%20%28double-precision%29))
  (Utilities|IsValid (Variables|Config|GetTrajectory)
    (:Is%20Valid
      (Variables|Default|SetTime (Math|Float|%(Float) (+ (Variables|Default|GetTime) (* DeltaSeconds (* (Variables|Default|GetSpeedMultiplier) 0.1))) 1.0))
      (Transformation|SetActorLocation (+ (Spline|GetLocationatTime (Variables|/Game/Task_05/BP_Trajectory.BP_Trajectory_C|GetSpline (Variables|Config|GetTrajectory)) (Variables|Default|GetTime) "World" false) "0.000000,0.000000,100.000000") false false))))

(fn UpdatePredictionPath
  (if (Variables|Default|GetbShouldUpdatePrediction)
    (bind (_predictresult _returnvalue) (Class|GameplayStatics|BlueprintPredictProjectilePathAdvanced (Utilities|Struct|MakePredictProjectilePathParams (Transformation|GetWorldLocation (Variables|Default|GetProjectileSpawnPoint)) (* (Math|Vector|GetForwardVector (Variables|Default|GetProjectileSpawnPoint)) (Variables|Default|GetLaunchVelocity)) true 25.0 1e+01 true "ECC_Camera" (Utilities|Array|MakeArray "ObjectTypeQuery1" "ObjectTypeQuery2") (Utilities|Array|MakeArray self) 5.0 0.0 "ForOneFrame")))
    (if _returnvalue
      (Transformation|SetActorLocationAndRotation (Variables|Default|GetHitPlace) (.ImpactPoint (Collision|BreakHitResult (.HitResult (Utilities|Struct|BreakPredictProjectilePathResult _predictresult)))) (Math|Rotator|MakeRotator 0.0 0.0 (.yaw (Transformation|GetActorRotation))))
      (Variables|Default|SetLastPredictionPathDuration (.Time (Utilities|Struct|BreakPredictProjectilePathPointData (.LastTraceDestination (Utilities|Struct|BreakPredictProjectilePathResult _predictresult))))))))
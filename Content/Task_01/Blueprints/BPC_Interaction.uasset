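; Actor component that lets its owner detect and interact with BPI_Interactable actors nearby.
; A sphere created at BeginPlay tracks interactables in range through overlaps.
; Each Tick filters them by Visibility line-of-sight trace from the owner, picks the nearest, and sends interface messages when they gain or lose focus.
; Interaction is triggered separately, by a range-compensated camera trace with the same reachability check, or forced on a given object.
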(event Custom|OnBeginOverlap
  (params (OverlappedComponent :type Primitive%20Component%20Object%20Reference) (OtherActor :type Actor%20Object%20Reference) (OtherComp :type Primitive%20Component%20Object%20Reference) (OtherBodyIndex :type Integer) (bFromSweep :type Boolean) (SweepResult :type Hit%20Result%20Structure%20%28by%20ref%29))
  (if (Utilities|DoesObjectImplementInterface OtherActor "/Game/Task_01/Blueprints/BPI_Interactable.BPI_Interactable_C")
    (Utilities|Array|AddUnique (Variables|Default|GetInteractableObjectsInRange) OtherActor)))

(event Custom|OnEndOverlap
  (params (OverlappedComponent :type Primitive%20Component%20Object%20Reference) (OtherActor :type Actor%20Object%20Reference) (OtherComp :type Primitive%20Component%20Object%20Reference) (OtherBodyIndex :type Integer))
  (if (Utilities|DoesObjectImplementInterface OtherActor "/Game/Task_01/Blueprints/BPI_Interactable.BPI_Interactable_C")
    (Utilities|Array|RemoveItem (Variables|Default|GetInteractableObjectsInRange) OtherActor)))

(event EventBeginPlay
  (CallFunction|CreateCollisionComponent))

(event EventTick
  (params (DeltaSeconds :type Float%20%28single-precision%29))
  (bind _reachableobjects (CallFunction|FilterReachebilityforObjects (Variables|Default|GetInteractableObjectsInRange)))
  (bind _returnvalue (CallFunction|FindMostAppropriateObjecttoInteract _reachableobjects))
  (Variables|Default|SetCurrentInteractableObject _returnvalue)
  (Utilities|FlowControl|Sequence
    (:then_0
      (if (and (Utilities|IsValid (Variables|Default|GetPreviousInteractableObject)) (!= (Variables|Default|GetPreviousInteractableObject) (Variables|Default|GetCurrentInteractableObject)))
        (Class|BPIInteractable|OnStoppedBeingInteractable(Message) (Variables|Default|GetPreviousInteractableObject))))
    (:then_1
      (Utilities|IsValid (Variables|Default|GetCurrentInteractableObject)
        (:Is%20Valid
          (Class|BPIInteractable|OnBecameInteractable(Message) (Variables|Default|GetCurrentInteractableObject)))))
    (:then_2
      (Variables|Default|SetPreviousInteractableObject (Variables|Default|GetCurrentInteractableObject)))))

(fn CreateCollisionComponent
  (bind _returnvalue (Game|AddComponentbyClass (Components|GetOwner) "/Script/Engine.SphereComponent" false))
  (Variables|Default|SetCollisionSphere _returnvalue)
  (Components|Sphere|SetSphereRadius (Variables|Default|GetCollisionSphere) (Variables|Default|GetInteractionRaduis) true)
  (Collision|SetCollisionResponsetoAllChannels (Variables|Default|GetCollisionSphere) "ECR_Overlap")
  (Collision|BindEventtoOnComponentBeginOverlap (Variables|Default|GetCollisionSphere) (EventDispatchers|CreateEvent :!event Custom|OnBeginOverlap))
  (Collision|BindEventtoOnComponentEndOverlap (Variables|Default|GetCollisionSphere) (EventDispatchers|CreateEvent :!event Custom|OnEndOverlap)))

(fn FilterReachebilityforObjects
  (params (InteractableObjects :type Array%20of%20Actor%20Object%20References))
  (for _array_element InteractableObjects
    (LocalVariables|SetObjectToTest _array_element)
    (bind _breachable (CallFunction|CheckIsObjectReachable (LocalVariables|GetObjectToTest)))
    (if _breachable
      (Utilities|Array|AddUnique (LocalVariables|GetResult) (LocalVariables|GetObjectToTest))))
  (return (LocalVariables|GetResult)))

(fn FindMostAppropriateObjecttoInteract
  (params (InteractableObjects :type Array%20of%20Actor%20Object%20References))
  (return (.ReturnValue (Actor|FindNearestActor (Transformation|GetActorLocation (Components|GetOwner)) InteractableObjects))))

(fn TryInteractwithTrace
  (params (CameraComponent :type Camera%20Component%20Object%20Reference))
  (bind _returnvalue (Transformation|GetWorldLocation CameraComponent))
  (bind (_outhit _returnvalue_2) (Collision|LineTraceByChannel _returnvalue (+ _returnvalue (* (Math|Vector|GetForwardVector CameraComponent) (+ (Variables|Default|GetInteractionRaduis) (Math|Vector|Distance(Vector) (Transformation|GetWorldLocation CameraComponent) (Transformation|GetActorLocation (Components|GetOwner)))))) "TraceTypeQuery1" false 0 "None"))
  (if _returnvalue_2
    (bind _breachable (CallFunction|CheckIsObjectReachable (.HitActor (Collision|BreakHitResult _outhit))))
    (if _breachable
      (Class|BPIInteractable|OnInteract(Message) (.HitActor (Collision|BreakHitResult _outhit))))))

(fn ForceInteractwithObject
  (params (Object :type Actor%20Object%20Reference))
  (Class|BPIInteractable|OnInteract(Message) Object))

(fn CheckIsObjectReachable
  (params (ObjectToTest :type Actor%20Object%20Reference))
  (bind _returnvalue (Collision|LineTraceByChannel (Transformation|GetActorLocation (Components|GetOwner)) (Transformation|GetActorLocation ObjectToTest) "TraceTypeQuery1" false (Utilities|Array|MakeArray (Components|GetOwner) ObjectToTest) "ForOneFrame"))
  (return (not _returnvalue)))
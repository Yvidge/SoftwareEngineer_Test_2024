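; BP_Controller is a player controller that sets up input and the on-screen HUD when play begins.
; BeginPlay runs two collapsed graphs: one adds the IMC_Input mapping context to the Enhanced Input local player subsystem.
; The other creates a W_HUD widget owned by the controller, stores it and adds it to the viewport.
; GetHUDWidget returns that stored widget.
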(event EventBeginPlay
  (|CG_AddInput)
  (|CG_AddHUD))

(fn ConstructionScript)

(fn GetHUDWidget
  (return (Variables|Default|GetHUD)))